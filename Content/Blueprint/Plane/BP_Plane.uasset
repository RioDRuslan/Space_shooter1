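; BP_Plane is a player-controlled plane Character that moves, climbs, descends and fires projectiles.
; On BeginPlay it adds the Moving Enhanced Input mapping context to the player's subsystem.
; Move, fly and down actions add movement input along fixed world X and Z axes, with the vertical ones switching CharacterMovement to Flying mode.
; The shoot action spawns BP_Projectile_Plane at the plane's location and rotation, owned by it.
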(event Input|EnhancedActionEvents|EnhancedInputActionAI_Move_Plane
  (params (ActionValue :type Float%20%28double-precision%29) (ElapsedSeconds :type Float%20%28double-precision%29) (TriggeredSeconds :type Float%20%28double-precision%29) (InputAction :type Input%20Action%20Object%20Reference :default "/Game/Blueprint/Plane/Input/AI_Move_Plane.AI_Move_Plane"))
  (Pawn|Input|AddMovementInput "0.300000,0.000000,0.000000" ActionValue false))

(event Input|EnhancedActionEvents|EnhancedInputActionAI_Shoot_Plane
  (params (ActionValue :type Boolean) (ElapsedSeconds :type Float%20%28double-precision%29) (TriggeredSeconds :type Float%20%28double-precision%29) (InputAction :type Input%20Action%20Object%20Reference :default "/Game/Blueprint/Plane/Input/AI_Shoot_Plane.AI_Shoot_Plane"))
  (bind _self self)
  (:Started
    (Game|SpawnActorfromClass "/Game/Blueprint/Projectiles/Plane/BP_Projectile_Plane.BP_Projectile_Plane_C" (Math|Transform|MakeTransform (Transformation|GetActorLocation) (Transformation|GetActorRotation) "1.000000,1.000000,1.000000") "AlwaysSpawn" "MultiplyWithRoot" _self _self)))

(event Input|EnhancedActionEvents|EnhancedInputActionAI_Fly
  (params (ActionValue :type Float%20%28double-precision%29) (ElapsedSeconds :type Float%20%28double-precision%29) (TriggeredSeconds :type Float%20%28double-precision%29) (InputAction :type Input%20Action%20Object%20Reference :default "/Game/Blueprint/Plane/Input/AI_Fly.AI_Fly"))
  (Pawn|Input|AddMovementInput "0.000000,0.000000,0.300000" ActionValue false)
  (Pawn|Components|CharacterMovement|SetMovementMode (Variables|Character|GetCharacterMovement) "MOVE_Flying" 0))

(event Input|EnhancedActionEvents|EnhancedInputActionAI_Down
  (params (ActionValue :type Float%20%28double-precision%29) (ElapsedSeconds :type Float%20%28double-precision%29) (TriggeredSeconds :type Float%20%28double-precision%29) (InputAction :type Input%20Action%20Object%20Reference :default "/Game/Blueprint/Plane/Input/AI_Down.AI_Down"))
  (Pawn|Input|AddMovementInput "0.000000,0.000000,-0.300000" 1.0 false)
  (Pawn|Components|CharacterMovement|SetMovementMode (Variables|Character|GetCharacterMovement) "MOVE_Flying" 0))

(event EventBeginPlay
  (bind _asplayer_controller (Utilities|Casting|CastToPlayerController (Pawn|GetController)))
  (Input|AddMappingContext (PlayerController|LocalPlayerSubsystems|GetEnhancedInputLocalPlayerSubsystem _asplayer_controller) "/Game/Blueprint/Plane/Input/Moving.Moving" 0 "(bIgnoreAllPressedKeysUntilRelease=True,bForceImmediately=False,bNotifyUserSettings=False)"))

(fn ConstructionScript)