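; AIC_Eye is the AI controller for the BP_Enemy_Eye enemy, steering it toward a target pawn.
; On possess it caches the pawn as the owning eye, and a SetTargetPlayer event supplies the target.
; Each tick, while both are valid, it feeds the forward vector of a look-at rotation into the eye's MoveTowards, giving direct pursuit without pathfinding.
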(event Custom|SetTargetPlayer
  (params (TargetPAwn :type Pawn%20Object%20Reference))
  (Variables|Default|SetTargetPAwn TargetPAwn))

(event EventTick
  (params (DeltaSeconds :type Float%20%28single-precision%29))
  (Utilities|IsValid (Variables|Default|GetOwningEye)
    (:Is%20Valid
      (Utilities|IsValid (Variables|Default|GetTargetPAwn)
        (:Is%20Valid
          (Default|MoveTowards (Variables|Default|GetOwningEye) (Math|Vector|GetForwardVector (Math|Rotator|FindLookatRotation (Transformation|GetActorLocation (Variables|Default|GetOwningEye)) (Transformation|GetActorLocation (Variables|Default|GetTargetPAwn)))) 1.0))))))

(event EventPossess
  (params (PossessedPawn :type Pawn%20Object%20Reference))
  (bind _asbp_enemy_eye (Utilities|Casting|CastToBP_Enemy_Eye PossessedPawn))
  (Variables|Default|SetOwningEye _asbp_enemy_eye))

(fn ConstructionScript
  (|CallParentFunction))