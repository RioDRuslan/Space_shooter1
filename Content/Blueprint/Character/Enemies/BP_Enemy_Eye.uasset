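; BP_Enemy_Eye is a flying eye enemy that detects the player and hands it to its AI controller as a target.
; The first player overlap with AggroRange passes the player to AIC_Eye and plays a detection sound, gated by a DoOnce that is never reset here.
; MoveTowards applies movement input and flips the actor 180 degrees according to the sign of the direction's X.
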(event OnComponentBeginOverlap(AggroRange)
  (params (OverlappedComponent :type Primitive%20Component%20Object%20Reference) (OtherActor :type Actor%20Object%20Reference) (OtherComp :type Primitive%20Component%20Object%20Reference) (OtherBodyIndex :type Integer) (bFromSweep :type Boolean) (SweepResult :type Hit%20Result%20Structure%20%28by%20ref%29))
  (bind _asbp_player (Utilities|Casting|CastToBP_Player OtherActor))
  (Utilities|FlowControl|DoOnce false
    (:Completed
      (bind _asaic_eye (Utilities|Casting|CastToAIC_Eye (AI|GetAIController self)))
      (Default|SetTargetPlayer _asaic_eye _asbp_player)
      (Audio|PlaySoundatLocation "/Game/Assets/Sounds/Detected_FlyEye_Cue.Detected_FlyEye_Cue" (Transformation|GetActorLocation) "0, 0, 0" 1.0 1.0 0.0 0 0 0 0))))

(event Custom|MoveTowards
  (params (WorldDirection :type Vector) (ScaleValue :type Float%20%28single-precision%29))
  (Pawn|Input|AddMovementInput WorldDirection ScaleValue false)
  (Transformation|SetActorRotation (select (< (.X (Math|Vector|BreakVector WorldDirection)) 0.0) "0.000000,180.000000,0.000000" "0, 0, 0")))

(event EventBeginPlay
  (|CallParentFunction) ; This node is disabled and will not be called.\nDrag off pins to build functionality.
)

(event Collision|EventActorBeginOverlap
  (params (OtherActor :type Actor%20Object%20Reference))
  (|CallParentFunction OtherActor) ; This node is disabled and will not be called.\nDrag off pins to build functionality.
)

(event EventTick
  (params (DeltaSeconds :type Float%20%28single-precision%29))
  (|CallParentFunction DeltaSeconds) ; This node is disabled and will not be called.\nDrag off pins to build functionality.
)

(fn ConstructionScript
  (|CallParentFunction))