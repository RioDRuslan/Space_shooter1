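; BP_Enemy_Crab is a 2D flipbook crab enemy that walks along its facing direction and turns at walls and ledges.
; A WalkForward event adds movement input along the forward vector, while wall-detector overlap begin and ledge-detector overlap end both call TurnCharacter, which is not defined here.
; Tick runs the parent logic, then UpdateAnim picks the walk or idle flipbook based on velocity.
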(event OnComponentBeginOverlap(Walldetector)
  (params (OverlappedComponent :type Primitive%20Component%20Object%20Reference) (OtherActor :type Actor%20Object%20Reference) (OtherComp :type Primitive%20Component%20Object%20Reference) (OtherBodyIndex :type Integer) (bFromSweep :type Boolean) (SweepResult :type Hit%20Result%20Structure%20%28by%20ref%29))
  (CallFunction|TurnCharacter))

(event OnComponentEndOverlap(LedgeDetector)
  (params (OverlappedComponent :type Primitive%20Component%20Object%20Reference) (OtherActor :type Actor%20Object%20Reference) (OtherComp :type Primitive%20Component%20Object%20Reference) (OtherBodyIndex :type Integer))
  (CallFunction|TurnCharacter))

(event Custom|WalkForward
  (params (ScaleValue :type Float%20%28single-precision%29))
  (Pawn|Input|AddMovementInput (Transformation|GetActorForwardVector) ScaleValue false))

(event EventBeginPlay
  (|CallParentFunction) ; This node is disabled and will not be called.\nDrag off pins to build functionality.
)

(event Collision|EventActorBeginOverlap
  (params (OtherActor :type Actor%20Object%20Reference))
  (|CallParentFunction OtherActor) ; This node is disabled and will not be called.\nDrag off pins to build functionality.
)

(event EventTick
  (params (DeltaSeconds :type Float%20%28single-precision%29))
  (|CallParentFunction DeltaSeconds)
  (CallFunction|UpdateAnim))

(fn ConstructionScript
  (|CallParentFunction))

(fn UpdateAnim
  (Sprite|SetFlipbook (Variables|Default|GetSprite) (select (> (Math|Vector|VectorLength (Transformation|GetVelocity)) 0.0) "/Game/Assets/Character/Enemies/crab/crab__Walk.crab__Walk" "/Game/Assets/Character/Enemies/crab/crab__Idle.crab__Idle")))